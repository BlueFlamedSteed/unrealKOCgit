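; BP_Switch is an actor that changes the look of its static mesh when another actor overlaps it.
; Overlap begin sets the first material slot to MyFirstMaterial, and overlap end sets it to M_Chair.
; The construction script applies a dynamic instance of M_Chair and stores it in TheColor, but the overlap events assign materials directly without using it.
; BeginPlay only prints a creation message.
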(event `self.ReceiveBeginPlay`
  (`KismetSystemLibrary.PrintText` "BP_Switch Created"))

(event `self.ReceiveTick`
  (params (DeltaSeconds :type "Float (single-precision)")))

(event `self.ReceiveActorBeginOverlap`
  (params (OtherActor :type "Actor Object Reference"))
  (`PrimitiveComponent.SetMaterial` (`self.StaticMesh`) 0 "/Game/Materials/MyFirstMaterial.MyFirstMaterial"))

(event `self.ReceiveActorEndOverlap`
  (params (OtherActor :type "Actor Object Reference"))
  (`PrimitiveComponent.SetMaterial` (`self.StaticMesh`) 0 "/Game/StarterContent/Props/Materials/M_Chair.M_Chair"))

(fn `UserConstructionScript`
  (bind _returnvalue (`PrimitiveComponent.CreateDynamicMaterialInstance` (`self.StaticMesh`) 0 "/Game/StarterContent/Props/Materials/M_Chair.M_Chair"))
  (set `self.TheColor` _returnvalue))